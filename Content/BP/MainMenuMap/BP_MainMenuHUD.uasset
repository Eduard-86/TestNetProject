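; Main menu HUD that displays the menu widget and relays the player's entered name to the controller.
; On BeginPlay it creates the widget, adds it to the viewport and binds to its editable text's commit event.
; Committed text is passed to BP_MainMenuController's EnteredPlayerName through the owning player, regardless of commit method.
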(event Custom|EditedNameFromWidget
  (params (Text :type Text%20%28by%20ref%29) (CommitMethod :type ETextCommit%20Enum :default "Default"))
  (bind _asbp_main_menu_controller (Utilities|Casting|CastToBP_MainMenuController (Variables|Default|GetPlayerOwner)))
  (Default|EnteredPlayerName _asbp_main_menu_controller Text))

(event EventBeginPlay
  (bind _returnvalue (UserInterface|CreateWidget (Variables|Default|GetMainWidgetClass) (Game|GetPlayerController 0)))
  (bind _output_get (Variables|Default|SetMainWidget (.AsUW%20Main%20Menu (Utilities|Casting|CastToUW_MainMenu _returnvalue))))
  (UserInterface|Viewport|AddtoViewport _output_get 0)
  (EventDispatchers|BindEventtoOnTextCommitted (Variables|/Game/BP/MainMenuMap/Widgets/UW_MainMenu.UW_MainMenu_C|GetEditableText _output_get) (delegate Custom|EditedNameFromWidget)))

(fn ConstructionScript)