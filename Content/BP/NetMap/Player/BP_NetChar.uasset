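; BP_NetChar is a networked player character Blueprint that performs a dodge roll on input.
; The roll input calls an RPC event that triggers a multicast, which plays a stand-to-roll montage at increased speed unless that montage is already active.
; An unconnected prototype keeps an alternative to replicated root motion, driving forward movement and walk speed from an animation curve.
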(event Custom|RPC_Roll
  (CallFunction|MultiRoll))

(event Custom|Multi_Roll
  (if (not (Class|AnimInstance|MontageIsActive (Components|SkeletalMesh|GetAnimInstance (Variables|Character|GetMesh))))
    (Animation|Montage|PlayMontage (Variables|Character|GetMesh) "/Game/Anim/Manny_StandToRoll_UE1_Montage.Manny_StandToRoll_UE1_Montage" 1.5)))

(event Input|EnhancedActionEvents|EnhancedInputActionIA_Roll
  (params (ActionValue :type Boolean) (ElapsedSeconds :type Float%20%28double-precision%29) (TriggeredSeconds :type Float%20%28double-precision%29) (InputAction :type Input%20Action%20Object%20Reference :default "/Game/ThirdPerson/Input/Actions/IA_Roll.IA_Roll"))
  (:Started
    (CallFunction|RPCRoll)))

(event EventTick
  (params (DeltaSeconds :type Float%20%28single-precision%29))
  ;[0.15 0.15 0.15 0.5] С рутами в репликации всё непросто, я решил остановиться на мультиксте. Это не идеальный подход, который может порождать лаг в проигрывании анимации, но при тестировании я его не заметил, что повлияло на конечное решение. Тут запечатлён второй подход, а именно его прототип: не использовать рут, а использовать кривые и логику в мув компоненте. Если бы выбор пал на неё, то можно было бы создать наследника и там реализовать логику перекатов, как это сделано с прыжком.
)

(fn ConstructionScript
  (|CallParentFunction))