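; BP_NetHUD creates the chat widget for the local player in the NetMap and relays sent messages to the player controller.
; On BeginPlay it checks that player controller 0 is local, adds the widget to the viewport and binds to the W_Chat OnMessageSent event.
; Each sent message is forwarded to GetMessage on BP_NetController, then input returns to game-only mode with a flush.
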(event Custom|GetMessage
  (params (Message :type Text))
  (bind _returnvalue (Game|GetPlayerController 0))
  (Default|GetMessage (.AsBP%20Net%20Controller (Utilities|Casting|CastToBP_NetController _returnvalue)) Message)
  (Input|SetInputModeGameOnly _returnvalue true))

(event EventBeginPlay
  (if (Pawn|IsLocalPlayerController (Game|GetPlayerController 0))
    (bind _returnvalue (UserInterface|CreateWidget (Variables|Default|GetMainWidget) (Game|GetPlayerController 0)))
    (bind _output_get (Variables|Default|SetChatWidget _returnvalue))
    (UserInterface|Viewport|AddtoViewport _output_get 0)
    (EventDispatchers|BindEventtoOnMessageSent (.AsUW%20Chat (Utilities|Casting|CastToUW_Chat _output_get)) (delegate Custom|GetMessage))))

(fn ConstructionScript)