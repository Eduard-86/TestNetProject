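; Networked player controller that links the local chat widget to the shared chat log in BP_NetGameState.
; Non-empty text from GetMessage is added to the game state directly on authority, or through a server event from clients.
; The local controller binds to the game state's new-message event and reprints the full message array in the HUD's UW_Chat widget.
; The IA_Message input focuses the chat text field.
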(event Custom|SendChatMessage
  (params (Message :type Text))
  (if (Ability|HasAuthority)
    (bind _asbp_net_game_state (Utilities|Casting|CastToBP_NetGameState (Game|GetGameState)))
    (Default|AddNewMessage _asbp_net_game_state self Message)
    (else
      (CallFunction|ServerSendChatMessage Message))))

(event Custom|Server_SendChatMessage
  (params (Message :type Text))
  (bind _asbp_net_game_state (Utilities|Casting|CastToBP_NetGameState (Game|GetGameState)))
  (Default|AddNewMessage _asbp_net_game_state self Message))

(event Custom|GetMessage
  (params (Text :type Text%20%28by%20ref%29))
  (if (Pawn|IsLocalPlayerController)
    (if (not (Utilities|Text|TextIsEmpty Text))
      (CallFunction|SendChatMessage Text))))

(event Custom|OtherAddMessage
  (bind _returnvalue (Game|GetGameState))
  (bind (_asbp_net_game_state _bsuccess) (Utilities|Casting|CastToBP_NetGameState _returnvalue))
  (if _bsuccess
    (bind _chatmessagearray (Default|GetMessageArray _asbp_net_game_state))
    (Default|PrintAllMesage (.AsUW%20Chat (Utilities|Casting|CastToUW_Chat (Variables|/Game/BP/NetMap/Player/BP_NetHUD.BP_NetHUD_C|GetChatWidget (.AsBP%20Net%20HUD (Utilities|Casting|CastToBP_NetHUD (HUD|GetHUD)))))) _chatmessagearray)))

(event EventBeginPlay
  (if (Pawn|IsLocalPlayerController)
    (EventDispatchers|BindEventtoEventAddNewMessage (.AsBP%20Net%20Game%20State (Utilities|Casting|CastToBP_NetGameState (Game|GetGameState))) (delegate Custom|OtherAddMessage))))

(event Input|EnhancedActionEvents|EnhancedInputActionIA_Message
  (params (ActionValue :type Boolean) (ElapsedSeconds :type Float%20%28double-precision%29) (TriggeredSeconds :type Float%20%28double-precision%29) (InputAction :type Input%20Action%20Object%20Reference :default "/Game/ThirdPerson/Input/Actions/IA_Message.IA_Message"))
  (:Started
    (Class|Widget|SetUserFocus (Variables|/Game/BP/NetMap/Player/Widgets/UW_Chat.UW_Chat_C|GetEditableText (.AsUW%20Chat (Utilities|Casting|CastToUW_Chat (Variables|/Game/BP/NetMap/Player/BP_NetHUD.BP_NetHUD_C|GetChatWidget (.AsBP%20Net%20HUD (Utilities|Casting|CastToBP_NetHUD (HUD|GetHUD))))))) self)))

(fn ConstructionScript)